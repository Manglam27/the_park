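; Master inventory Blueprint that stores items in a tile grid and selects among four quick slots by input.
; Items live in a flat array, with each item filling every tile its dimensions cover.
; Adding scans for free space, retrying once rotated, while stacked adds merge into same-name items or fall back to placement.
; Changes set a dirty flag, which Tick turns into an inventory-changed call.
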(event `self.ReceiveBeginPlay`
  (`KismetArrayLibrary.Array_Resize` (`self.Items`) (* (`self.Column`) (`self.Rows`))))

(event `self.ReceiveTick`
  (params (DeltaSeconds :type "Float (single-precision)"))
  (if (`self.IsDirty`)
    (set `self.IsDirty` false)
    (`self.On inventory changed`)))

(event `InputAction|QuickSlot_1`
  (params (Key :type "Key Structure"))
  (:`Pressed`
    (set `self.Active slot` "NewEnumerator0")
    (`self.Update Quick slots`)))

(event `InputAction|QuickSlot_2`
  (params (Key :type "Key Structure"))
  (:`Pressed`
    (set `self.Active slot` "NewEnumerator1")
    (`self.Update Quick slots`)))

(event `InputAction|QuickSlot_3`
  (params (Key :type "Key Structure"))
  (:`Pressed`
    (set `self.Active slot` "NewEnumerator2")
    (`self.Update Quick slots`)))

(event `InputAction|QuickSlot_4`
  (params (Key :type "Key Structure"))
  (:`Pressed`
    (set `self.Active slot` "NewEnumerator3")
    (`self.Update Quick slots`)))

(fn `Add Stacked Item`
  (params (`item object` :type "/Game/Main/Inventory/NEW_UIS/BP/BP_Item_Uobject Object Reference"))
  (returns (Result :type Boolean))
  (locals (`item (local)` :type "/Game/Main/Inventory/NEW_UIS/BP/BP_Item_Uobject Object Reference") (`Item Found` :type Boolean :default false))
  (bind _item__local_ (`local.item (local)`))
  (bind _returnvalue (+ (`/Game/Main/Inventory/NEW_UIS/BP/BP_Item_Uobject.Stack To add` (`local.item object`)) (`/Game/Main/Inventory/NEW_UIS/BP/BP_Item_Uobject.Current Stack` (`local.item (local)`))))
  (for _array_element (`self.Items`)
    (`/Engine/EditorBlueprintResources/StandardMacros.IsValid` _array_element
      (:`Is Valid`
        (set `local.Item Found` (`KismetTextLibrary.EqualEqual_TextText` (`/Game/Main/Inventory/NEW_UIS/BP/BP_Item_Uobject.Name` _array_element) (`/Game/Main/Inventory/NEW_UIS/BP/BP_Item_Uobject.Name` `item object`)))
        (if (<= (+ (`/Game/Main/Inventory/NEW_UIS/BP/BP_Item_Uobject.Current Stack` _array_element) (`/Game/Main/Inventory/NEW_UIS/BP/BP_Item_Uobject.Stack To add` `item object`)) (`/Game/Main/Inventory/NEW_UIS/BP/BP_Item_Uobject.Max Stack Amount` _array_element))
          (set `local.item (local)` _array_element)
          (break)))))
  (if (`local.Item Found`)
    (`/Engine/EditorBlueprintResources/StandardMacros.IsValid` _item__local_
      (:`Is Valid`
        (if (<= _returnvalue (`/Game/Main/Inventory/NEW_UIS/BP/BP_Item_Uobject.Max Stack Amount` (`local.item object`)))
          (set `/Game/Main/Inventory/NEW_UIS/BP/BP_Item_Uobject.Current Stack` _returnvalue _item__local_)
          (set `self.IsDirty` true)
          (return true)
          (else
            (bind _added (`self.Try ADD Item` (`local.item object`)))
            (return _added)))))
    (else
      (bind _added_2 (`self.Try ADD Item` (`local.item object`)))
      (return _added_2))))

(fn `ADDItemAt`
  (params (`Item object` :type "/Game/Main/Inventory/NEW_UIS/BP/BP_Item_Uobject Object Reference") (`Top left index` :type Integer))
  (bind _tile (`self.For each Index` `Item object` `Top left index`)
    (:`LoopBody`
      (`KismetArrayLibrary.Array_Set` (`self.Items`) (`self.Tile to index` _tile) (`local.Item object`)))
    (:`Completed`
      (set `self.IsDirty` true))))

(fn `Get all Items`
  (returns (`All Items` :type "Map of /Game/Main/Inventory/NEW_UIS/BP/BP_Item_Uobject Object Reference to /Game/Main/Inventory/NEW_UIS/ST_Tile Structure"))
  (locals (`All Items (local)` :type "Map of /Game/Main/Inventory/NEW_UIS/BP/BP_Item_Uobject Object Reference to /Game/Main/Inventory/NEW_UIS/ST_Tile Structure") (`Current Item (locol)` :type "/Game/Main/Inventory/NEW_UIS/BP/BP_Item_Uobject Object Reference"))
  (for (_array_element _array_index) (`self.Items`)
    (bind _output_get (set `local.Current Item (locol)` _array_element))
    (`/Engine/EditorBlueprintResources/StandardMacros.IsValid` _output_get
      (:`Is Valid`
        (if (not (`BlueprintMapLibrary.Map_Contains` (`local.All Items (local)`) _array_element))
          (`BlueprintMapLibrary.Map_Add` (`local.All Items (local)`) (`local.Current Item (locol)`) (`self.Index to Tile` _array_index))))))
  (return (`local.All Items (local)`)))

(fn `Get Item at index`
  (params (Index :type Integer))
  (returns (Valid :type Boolean) (`Item Object` :type "/Game/Main/Inventory/NEW_UIS/BP/BP_Item_Uobject Object Reference"))
  (if (`KismetArrayLibrary.Array_IsValidIndex` (`self.Items`) Index)
    (return true (`|GetArrayItem` (`self.Items`) (`local.Index`)))
    (else
      (return false null))))

(fn `Index to Tile`
  (params (Index :type Integer))
  (returns (Tile :type "/Game/Main/Inventory/NEW_UIS/ST_Tile Structure"))
  (bind _column (`self.Column`))
  (return (make `/Game/Main/Inventory/NEW_UIS/ST_Tile` (mod Index _column) (/ Index _column))))

(fn `IsRoomAvailable`
  (params (`Item Object` :type "/Game/Main/Inventory/NEW_UIS/BP/BP_Item_Uobject Object Reference") (`Top Left Index` :type Integer))
  (returns (Result :type Boolean))
  (`|ExecutionSequence`
    (:`then_0`
      (bind _tile (`self.For each Index` `Item Object` `Top Left Index`)
        (:`LoopBody`
          (`self.IsTileValid` _tile
            (:`true`
              (bind (_valid _item_object) (`self.Get Item at index` (`self.Tile to index` _tile)))
              (if _valid
                (if (`KismetSystemLibrary.IsValid` _item_object)
                  (return false))
                (else
                  (return false))))
            (:`false`
              (return false))))))
    (:`then_1`
      (return true))))

(fn `Remove item`
  (params (`Item Object` :type "/Game/Main/Inventory/NEW_UIS/BP/BP_Item_Uobject Object Reference"))
  (`/Engine/EditorBlueprintResources/StandardMacros.IsValid` `Item Object`
    (:`Is Valid`
      (for (_array_element _array_index) (`self.Items`)
        (if (== _array_element (`local.Item Object`))
          (`KismetArrayLibrary.Array_Set` (`self.Items`) _array_index)
          (set `self.IsDirty` true))))))

(fn `Tile to index`
  (params (Tile :type "/Game/Main/Inventory/NEW_UIS/ST_Tile Structure"))
  (returns (Index :type Integer))
  (return (+ Tile_x_2_6B042A8F43562459CC4A588EB82EDFFD (* Tile_Y_4_4AC9147E478D4C1848749EB67F4D0086 (`self.Column`)))))

(fn `Try ADD Item`
  (params (`Item object` :type "/Game/Main/Inventory/NEW_UIS/BP/BP_Item_Uobject Object Reference"))
  (returns (Added :type Boolean))
  (`/Engine/EditorBlueprintResources/StandardMacros.IsValid` `Item object`
    (:`Is Valid`
      (for (_ _array_index) (`self.Items`) :!label _label
        (bind _result (`self.IsRoomAvailable` (`local.Item object`) _array_index))
        (if _result
          (`self.ADDItemAt` (`local.Item object`) _array_index)
          (return true)))
      ;[0 0 0] Auto Rotation.
      (`|ExecutionSequence`
        (:`then_0`
          (`/Engine/EditorBlueprintResources/StandardMacros.DoOnce` false
            (:`Completed`
              (`/Game/Main/Inventory/NEW_UIS/BP/BP_Item_Uobject.Rotate` (`local.Item object`))
              (goto _label))))
        (:`then_1`
          (`/Game/Main/Inventory/NEW_UIS/BP/BP_Item_Uobject.Rotate` (`local.Item object`))
          (return false))))))