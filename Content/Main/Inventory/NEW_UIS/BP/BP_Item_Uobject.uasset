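; BP_Item_Uobject is a data object for an inventory item, holding its class, icons, dimensions and rotation state.
; Rotate toggles a Rotated flag, which the getters read to return either the normal or rotated icon and to swap the X and Y dimensions.
; The name and dimension handling point to use in a grid-based inventory UI where items can be turned.
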(fn `Get Dimension`
  (returns (Dimension :type "IntPoint Structure"))
  (bind (_dimension_x _dimension_y) (break `IntPoint` (`self.Dimension`)))
  (if (`self.Rotated`)
    (return (make `IntPoint` _dimension_y _dimension_x))
    (else
      (return (`self.Dimension`)))))

(fn `Get Icons`
  (returns (Icon :type "MaterialInterface Object Reference"))
  (return (select `bool` (`self.Rotated`) :`false` (`self.Icon`) :`true` (`self.Icon_Rotated`))))

(fn `Get item class`
  (returns (`Item class` :type "/Game/Main/Inventory/NEW_UIS/BP/Main_Item_Actor Class Reference"))
  (return (`self.Item class`)))

(fn `Is Rotated`
  (returns (Rotated :type Boolean))
  (return (`self.Rotated`)))

(fn `Rotate`
  (set `self.Rotated` (not (`self.Rotated`))))